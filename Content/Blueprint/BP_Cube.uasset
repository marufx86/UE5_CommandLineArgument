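; Cube actor that tests launch command-line arguments by recolouring its mesh and printing debug strings.
; On BeginPlay it compares the whole command line to "green" or "red" and sets the matching material, leaving it unchanged otherwise.
; Three disconnected experimental chains, which never run, check for an "-adminkey=" argument and pick green, red or white, trying LeftChop and exact-match comparisons against a hardcoded key.
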(event EventBeginPlay
  (bind _cube (Variables|Default|Getcube))
  ;[0.001452 0.15 0] Working only checking green and red
  (bind _returnvalue (Utilities|GetCommandLine))
  (Development|PrintString _returnvalue true true "(R=0.000000,G=0.660000,B=1.000000,A=1.000000)" 1e+02)
  (if (Utilities|Enum|Equal(Enum) _returnvalue "green")
    (Development|PrintString "True=Green" true true "(R=0.000000,G=0.660000,B=1.000000,A=1.000000)" 1e+02)
    (Rendering|Material|SetMaterial _cube 0 (Variables|Default|GetGreenMaterial%20))
    (elif (Utilities|Enum|Equal(Enum) _returnvalue "red")
      (Development|PrintString "False=Red" true true "(R=0.000000,G=0.660000,B=1.000000,A=1.000000)" 1e+02)
      (Rendering|Material|SetMaterial _cube 0 (Variables|Default|GetRedMaterial%20)))))

(fn ConstructionScript)